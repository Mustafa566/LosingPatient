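; Interactable computer that opens the main interface widget and supplies random patient records to it or other listeners.
; Interact toggles the widget, cursor and input mode if the player has a chair reference, disabling movement on open; otherwise it shows a SitOnChair widget.
; getPatientData picks a random ClientTable row from those not filtered by UserFilerID, stores it and calls CallUpdateNewUser.
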(event `disableMovement`
  (bind _asmy_player (cast `/Game/gamePlay/characters/myPlayer` (`GameplayStatics.GetPlayerPawn` 0)))
  (`self.DisableInput` _asmy_player (`GameplayStatics.GetPlayerController` 0)))

(event `turnPcOn`
  ;[1 0 0] Comment
  (set `PlayerController.bShowMouseCursor` true (`GameplayStatics.GetPlayerController` 0))
  (bind _returnvalue (`|CreateWidget` "/Game/gamePlay/widget/pcWidget.pcWidget_C"))
  (bind _output_get (set `self.pcWidget` _returnvalue))
  (`UserWidget.AddToViewport` _output_get 0))

(event `enableMovement`
  (bind _asmy_player (cast `/Game/gamePlay/characters/myPlayer` (`GameplayStatics.GetPlayerPawn` 0)))
  (`self.EnableInput` _asmy_player (`GameplayStatics.GetPlayerController` 0)))

(event `self.ReceiveBeginPlay`
  ;[1 1 1] Create Main Widget (BP_Computer)
  (bind _returnvalue (`|CreateWidget` "/Game/gamePlay/widget/Main_ComputerInterface/WB_MainInterface.WB_MainInterface_C"))
  (set `self.WB_MainWidget` _returnvalue))

(event `removeFromParent`
  ;[1 1 1] Remove parent / don't show cursor
  (set `PlayerController.bShowMouseCursor` false (`GameplayStatics.GetPlayerController` 0))
  (`Widget.RemoveFromParent` (`self.WB_MainWidget`)))

(event `/Game/gamePlay/actors/BP_ComputerInterface.Interact`
  (params (InteractingPlayer :type "/Game/gamePlay/characters/myPlayer Object Reference"))
  ;[1 1 1] Create Main Widget (BP_Computer)
  (`self.CheckWidgetAvailability` InteractingPlayer))

(event `getPatientData`
  (bind _userlist (`self.UserList`))
  (bind _returnvalue (`KismetMathLibrary.RandomIntegerInRange` 0 (- (`KismetArrayLibrary.Array_Length` _userlist) 1)))
  ;[1 1 1] Get patient data
  (bind _outrownames (`DataTableFunctionLibrary.GetDataTableRowNames` "/Game/gamePlay/clientTable.clientTable"))
  (`KismetArrayLibrary.Array_Clear` (`self.UserList`))
  (for (_array_element _array_index) _outrownames
    (if (not (`KismetArrayLibrary.Array_Contains` (`self.UserFilerID`) _array_index))
      (`KismetArrayLibrary.Array_Add` (`self.UserList`) _array_element)))
  (bind _returnvalue_2 (`|GetDataTableRow` "/Game/gamePlay/clientTable.clientTable" (`|GetArrayItem` _userlist _returnvalue))
    (:`then`
      (`KismetArrayLibrary.Array_Add` (`self.UserFilerID`) _returnvalue)
      (set `self.RandomUserData` _returnvalue_2)
      (`self.UpdateNewUser`))))

(fn `UserConstructionScript`)