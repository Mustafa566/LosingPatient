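; BP_Computer is an interactable computer actor that opens the main interface widget and supplies patient data.
; BeginPlay creates the widget; Interact toggles it and player input if the player's chair widget reference is valid, otherwise showing a SitOnChair widget.
; getPatientData takes the first ClientTable row not yet in UserList, records it and calls CallUpdateNewUser; despite the RandomUserData name, selection is sequential.
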(event `removeFromParent`
  ;[1 1 1] Remove parent / don't show cursor
  (set `PlayerController.bShowMouseCursor` false (`GameplayStatics.GetPlayerController` 0))
  (`Widget.RemoveFromParent` (`self.WB_MainWidget`)))

(event `/Game/gamePlay/actors/BP_ComputerInterface.Interact`
  (params (InteractingPlayer :type "/Game/gamePlay/characters/myPlayer Object Reference"))
  ;[1 1 1] Create Main Widget (BP_Computer)
  (`self.CheckWidgetAvailability` InteractingPlayer))

(event `disableMovement`
  (bind _asmy_player (cast `/Game/gamePlay/characters/myPlayer` (`GameplayStatics.GetPlayerPawn` 0)))
  (`self.DisableInput` _asmy_player (`GameplayStatics.GetPlayerController` 0)))

(event `enableMovement`
  (bind _asmy_player (cast `/Game/gamePlay/characters/myPlayer` (`GameplayStatics.GetPlayerPawn` 0)))
  (`self.EnableInput` _asmy_player (`GameplayStatics.GetPlayerController` 0)))

(event `self.ReceiveBeginPlay`
  ;[1 1 1] Create Main Widget (BP_Computer)
  (bind _returnvalue (`|CreateWidget` "/Game/gamePlay/widget/Main_ComputerInterface/WB_MainInterface.WB_MainInterface_C"))
  (bind _output_get (set `self.WB_MainWidget` _returnvalue))
  (`UserWidget.AddToViewport` _output_get 0))

(event `getPatientData`
  (bind _userlist (`self.UserList`))
  (bind _newuser (`self.NewUser`))
  ;[1 1 1] Get patient data
  (bind _outrownames (`DataTableFunctionLibrary.GetDataTableRowNames` "/Game/gamePlay/clientTable.clientTable"))
  (for _array_element _outrownames
    (if (`KismetArrayLibrary.Array_Contains` _userlist _array_element)
      (set `self.NewUser` "None")
      (set `self.RandomUserData` (struct))
      (else
        (set `self.NewUser` _array_element)
        (break))))
  (`KismetArrayLibrary.Array_Add` _userlist _newuser)
  (bind _returnvalue (`|GetDataTableRow` "/Game/gamePlay/clientTable.clientTable" _newuser)
    (:`then`
      (set `self.RandomUserData` _returnvalue)
      (`self.UpdateNewUser`))))

(fn `UserConstructionScript`)